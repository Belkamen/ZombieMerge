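; Tamed enemy character in ZombieMerge that takes damage, dies and attacks a supplied list of enemies.
; Attack stores the targets and starts a randomly timed looping timer, apparently for AttackEnemy, which only debug-traces toward a random target without using the hit.
; Non-lethal damage spawns a flesh impact and briefly interrupts attacking.
; Lethal damage clears StillAlive, which Tick detects to tag it Killed and run KillEvent once, stopping attacks.
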(event `self.ReceiveAnyDamage`
  (params (Damage :type "Float (single-precision)") (DamageType :type "DamageType Object Reference") (InstigatedBy :type "Controller Object Reference") (DamageCauser :type "Actor Object Reference"))
  (bind (_worldloc_x _worldloc_y _worldloc_z) (`KismetMathLibrary.BreakVector` (`self.WorldLoc`)))
  (bind _returnvalue (- (`self.Health`) Damage))
  (`|ExecutionSequence`
    (:`then_0`
      (if (`self.StillAlive?`)
        (set `self.WorldLoc` (`SceneComponent.K2_GetComponentLocation` (`self.CapsuleComponent`)))
        (if (<= _returnvalue 0.0)
          (set `self.StillAlive?` false)
          (else
            (set `self.Health` (`KismetMathLibrary.FTrunc` _returnvalue))
            (`GameplayStatics.SpawnEmitterAtLocation` "/Game/bulletvfx/Particles/VFX_Impact_Flesh.VFX_Impact_Flesh" (`KismetMathLibrary.MakeVector` _worldloc_x _worldloc_y (+ _worldloc_z 50.0)) (struct :`Pitch` 90.0))
            (set `self.isGettingHit?` true)
            ;[1 1 1] Pereriv pri poluchenii urona
            (`KismetSystemLibrary.K2_ClearAndInvalidateTimerHandle` (`self.AttackTimer`))
            (`KismetSystemLibrary.Delay` 0.2)
            (`self.StartAttack`)))
        (else
          (set `self.StillAlive?` false))))))

(event `self.ReceiveTick`
  (params (DeltaSeconds :type "Float (single-precision)"))
  (if (not (`self.StillAlive?`))
    (set `self.Tags` (`|MakeArray` "Killed" "Killed" :!type "Name"))
    (`/Engine/EditorBlueprintResources/StandardMacros.DoOnce` false
      (:`Completed`
        (set `self.isGettingHit?` false)
        (`self.KillEvent`)))))

(event `KillEvent`
  (bind (_worldloc_x _worldloc_y _worldloc_z) (`KismetMathLibrary.BreakVector` (`self.WorldLoc`)))
  (`GameplayStatics.SpawnEmitterAtLocation` "/Game/bulletvfx/Particles/VFX_Impact_Flesh.VFX_Impact_Flesh" (`KismetMathLibrary.MakeVector` _worldloc_x _worldloc_y (+ _worldloc_z 50.0)) (struct :`Pitch` 90.0))
  ;[1 1 1] AttackOff
  (`KismetSystemLibrary.K2_ClearAndInvalidateTimerHandle` (`self.AttackTimer`)))

(event `AttackEnemy`
  (bind _enemy (`self.Enemy`))
  ;[1 1 1] LogicaAttacki
  (bind _outhit (`KismetSystemLibrary.LineTraceSingleForObjects` :`Start` (`self.K2_GetActorLocation`) :`End` (`self.K2_GetActorLocation` (`|GetArrayItem` _enemy (`KismetMathLibrary.RandomInteger` (`KismetArrayLibrary.Array_LastIndex` _enemy)))) :`ObjectTypes` (`|MakeArray` "ObjectTypeQuery3" :!type "EObjectTypeQuery Enum") :`DrawDebugType` "ForDuration" :`DrawTime` 0.5)))

(event `/Game/BP_AttackEnemy.Attack`
  (params (Enemy :type "Array of Actor Object Reference (by ref)"))
  ;[1 1 1] StartAttacki
  (set `self.Enemy` Enemy)
  (`self.StartAttack`))

(event `StartAttack`
  ;[1 1 1] TimerAttacki
  (bind _returnvalue (`KismetSystemLibrary.K2_SetTimerDelegate` (`|CreateDelegate` :!event `AttackEnemy`) (`KismetMathLibrary.RandomFloatInRange` 0.3 0.5) true))
  (set `self.AttackTimer` _returnvalue))

(fn `UserConstructionScript`
  (set `self.Tags` (`self.ActorTags`)))