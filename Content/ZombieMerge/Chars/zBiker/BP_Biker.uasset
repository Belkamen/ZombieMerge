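; BP_Biker is a biker character in ZombieMerge that cheers periodically until the boss wall is gone.
; BeginPlay caches the actor tagged BossWall and runs a self-re-entering DoN loop that briefly pulses LetsYahoo, resetting after CountYahoo passes.
; Tick watches the wall reference and, once it is invalid, clears LetsYahoo and latches LetsFallDown, blocking further cheers.
; A ChangeRotation helper yaws the biker toward a given actor with a 90-degree offset.
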(event `self.ReceiveBeginPlay`
  ;[0.2654 1 0.7774] Do N Times with Delay
  (`|ExecutionSequence`
    (:`then_0`
      (bind _counter (`/Engine/EditorBlueprintResources/StandardMacros.Do N` (`self.CountYahoo`) :!label _label)
        (:`Exit`
          (`self.SetYahooOnEvent`)
          (`KismetSystemLibrary.Delay` 10.0)
          (if (== _counter (`self.CountYahoo`))
            (`|ExecutionSequence`
              (:`then_0`
                (`KismetSystemLibrary.PrintString` "End LOOP" true true (struct :`R` 1.0 :`G` 0.033549 :`B` 0.153251 :`A` 1.0)))
              (:`then_1`
                (goto _label :!via `Reset`)))
            (else
              (goto _label))))))
    (:`then_1`
      (bind _outactors (`GameplayStatics.GetAllActorsWithTag` "BossWall"))
      (set `self.BossWallRef` (`|GetArrayItem` _outactors)))))

(event `SetYahooOnEvent`
  ;[0.2865 0.2865 0.2865] Do Yahoo
  (if (not (`self.LetsFallDown`))
    (set `self.LetsYahoo` true)
    (`KismetSystemLibrary.Delay` 3.0)
    (set `self.LetsYahoo` false)))

(event `self.ReceiveTick`
  (params (DeltaSeconds :type "Float (single-precision)"))
  (`|ExecutionSequence`
    (:`then_0`
      (`/Engine/EditorBlueprintResources/StandardMacros.IsValid` (`self.BossWallRef`)
        (:`Is Not Valid`
          (`/Engine/EditorBlueprintResources/StandardMacros.DoOnce` false
            (:`Completed`
              (set `self.LetsYahoo` false)
              (set `self.LetsFallDown` true))))))))

(fn `ChangeRotation`
  (params (Actor :type "Actor Object Reference"))
  (`self.K2_SetActorRotation` (`KismetMathLibrary.MakeRotator` 0.0 0.0 (- (.yaw (`KismetMathLibrary.FindLookAtRotation` (`self.K2_GetActorLocation`) (`self.K2_GetActorLocation` Actor))) 90.0)))
  (return))

(fn `UserConstructionScript`)