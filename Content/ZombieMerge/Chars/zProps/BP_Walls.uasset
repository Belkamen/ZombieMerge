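; BP_Walls is a damageable wall prop with a configurable brick mesh, health and tags, the mesh and tags being applied in the construction script.
; AnyDamage lowers WallHealth, spawning a sand impact effect on non-lethal hits and clearing StillAlive on a lethal one, with debug prints.
; Tick polls StillAlive and once triggers destruction, which spawns the selected destruction actor at the mesh location and destroys the wall.
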(event `self.ReceiveAnyDamage`
  (params (Damage :type "Float (single-precision)") (DamageType :type "DamageType Object Reference") (InstigatedBy :type "Controller Object Reference") (DamageCauser :type "Actor Object Reference"))
  (bind (_returnvalue_x _returnvalue_y _returnvalue_z) (`KismetMathLibrary.BreakVector` (`SceneComponent.K2_GetComponentLocation` (`self.BrickMesh`))))
  (bind _returnvalue (- (`self.WallHealth`) Damage))
  (`|ExecutionSequence`
    (:`then_0`
      (if (`self.StillAlive?`)
        (set `self.WorldLoc` (`SceneComponent.K2_GetComponentLocation` (`self.BrickMesh`)))
        (if (<= _returnvalue 0.0)
          (set `self.StillAlive?` false)
          (else
            (set `self.WallHealth` (`KismetMathLibrary.FTrunc` _returnvalue))
            (`GameplayStatics.SpawnEmitterAtLocation` "/Game/bulletvfx/Particles/VFX_Impact_SandMassive.VFX_Impact_SandMassive" (`KismetMathLibrary.MakeVector` _returnvalue_x _returnvalue_y (+ _returnvalue_z 50.0)) (struct :`Pitch` 90.0) (1.0 1.0 1.0) true "AutoRelease")
            (`|ExecutionSequence`
              (:`then_1`
                (`KismetSystemLibrary.PrintString` "WallTakingDamage" true true (struct :`R` 1.0 :`G` 0.78671 :`A` 1.0))))))
        (else
          (set `self.StillAlive?` false))))
    (:`then_1`
      (`KismetSystemLibrary.PrintString` (`KismetStringLibrary.Conv_DoubleToString` Damage) true true (struct :`R` 0.472253 :`B` 0.510417 :`A` 1.0)))))

(event `self.ReceiveTick`
  (params (DeltaSeconds :type "Float (single-precision)"))
  (if (not (`self.StillAlive?`))
    (`/Engine/EditorBlueprintResources/StandardMacros.DoOnce` false
      (:`Completed`
        (`self.DestroyWallEvent`)))))

(event `DestroyWallEvent`
  (bind _brickmesh (`self.BrickMesh`))
  (set `self.WorldLoc` (`SceneComponent.K2_GetComponentLocation` _brickmesh))
  (`ActorComponent.K2_DestroyComponent` _brickmesh)
  (set `self.Tags_0` (`|MakeArray` "Killed" "Killed" :!type "Name"))
  (`|SpawnActorFromClass` (`self.SelectSpawnDestr`) (`KismetMathLibrary.MakeTransform` (`self.WorldLoc`) (struct :`Yaw` -90.0)) "Undefined" "OverrideRootScale" null null)
  (`self.K2_DestroyActor`))

(fn `UserConstructionScript`
  (`StaticMeshComponent.SetStaticMesh` (`self.BrickMesh`) (`self.SetMesh`))
  (set `self.Tags` (`self.Tags_0`)))